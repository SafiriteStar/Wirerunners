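; BP_FinalItem is the hackable final item, which triggers the enemy chase when hacked.
; StartHack passes the passkey from its BPCHackable component to the interactor's BPCHackMinigame, with itself as the target.
; HackSuccess finds BP_MainEnemyController in the world and calls StartChasing, while HackFailure generates a new passkey.
; Getter functions expose the component's hackable state and passkey, and both outcomes print debug messages.
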(event `self.StartHack`
  (params (Interactor :type "/Game/FirstPerson/Blueprints/BP_FirstPersonCharacter Object Reference"))
  (bind _currentpasskey (`/Game/Blueprints/UI/BPC_Hackable.GetPasskey` (`self.BPC_Hackable`)))
  (`/Game/Blueprints/UI/BPC_HackMinigame.StartHacking` (`/Game/FirstPerson/Blueprints/BP_FirstPersonCharacter.BPC_HackMinigame` Interactor) _currentpasskey self))

(event `self.HackSuccess`
  (`KismetSystemLibrary.PrintString` "Success Hacking")
  (bind _returnvalue (`GameplayStatics.GetActorOfClass` "/Game/FirstPerson/Blueprints/BP_MainEnemyController.BP_MainEnemyController_C"))
  (`/Engine/EditorBlueprintResources/StandardMacros.IsValid` _returnvalue
    (:`Is Valid`
      (`/Game/FirstPerson/Blueprints/BP_MainEnemyController.Start Chasing` _returnvalue))))

(event `self.HackFailure`
  (`KismetSystemLibrary.PrintString` "Failure Hacking")
  (`/Game/Blueprints/UI/BPC_Hackable.GenerateNewPasskey` (`self.BPC_Hackable`)))

(fn `GetHackable`
  (returns (IsHackable :type Boolean))
  (return (`/Game/Blueprints/UI/BPC_Hackable.IsHackable` (`self.BPC_Hackable`))))

(fn `GetHackPasskey`
  (returns (HackPasskey :type Integer))
  (bind _currentpasskey (`/Game/Blueprints/UI/BPC_Hackable.GetPasskey` (`self.BPC_Hackable`)))
  (return _currentpasskey))

(fn `UserConstructionScript`)